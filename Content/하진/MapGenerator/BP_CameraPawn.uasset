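; BP_CameraPawn is a camera pawn that moves by hold-and-drag input.
; Enhanced Input IA_Hold sets and clears an IsHolded flag, which gates IA_Drag.
; While held, the drag value is multiplied by the Arrow component's forward vector and a negative factor, then applied as an unswept local actor offset.
; Leftover Camvector and branch nodes never run.
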(event `EnhancedInput|/Game/하진/MapGenerator/Input/Action/IA_Hold`
  (params (ActionValue :type Boolean) (ElapsedSeconds :type "Float (double-precision)") (TriggeredSeconds :type "Float (double-precision)") (InputAction :type "InputAction Object Reference" :default "/Game/하진/MapGenerator/Input/Action/IA_Hold.IA_Hold"))
  (:`Started`
    (set `self.isHolded` true))
  (:`Completed`
    (set `self.isHolded` false)))

(event `EnhancedInput|/Game/하진/MapGenerator/Input/Action/IA_Drag`
  (params (ActionValue :type "Float (double-precision)") (ElapsedSeconds :type "Float (double-precision)") (TriggeredSeconds :type "Float (double-precision)") (InputAction :type "InputAction Object Reference" :default "/Game/하진/MapGenerator/Input/Action/IA_Drag.IA_Drag"))
  (:`Triggered`
    (if (`self.isHolded`)
      (`self.K2_AddActorLocalOffset` (* ActionValue (`SceneComponent.GetForwardVector` (`self.Arrow`)) -10.0)))))

(fn `UserConstructionScript`)